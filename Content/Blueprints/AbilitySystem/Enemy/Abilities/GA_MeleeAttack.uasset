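; Enemy melee attack gameplay ability that turns the avatar toward its combat target and plays a random tagged attack montage.
; A gameplay event matching the montage's tag triggers the hit, gathering live players in a small sphere at that tag's combat socket.
; It damages those who are not friends, then ends, and also ends if the montage completes, is interrupted or is cancelled.
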(event `self.K2_ActivateAbility`
  (bind _returnvalue (`self.GetAvatarActorFromActorInfo`))
  (bind _returnvalue_2 (`self.GetAvatarActorFromActorInfo`))
  (bind _taggedmontage_montage (break `TaggedMontage` (`self.TaggedMontage`)))
  (bind (_taggedmontage_montage_2 _taggedmontage_montagetag) (break `TaggedMontage` (`self.TaggedMontage`)))
  (bind _asenemy_interface (cast `EnemyInterface` _returnvalue_2))
  (bind _returnvalue_3 (`EnemyInterface.GetCombatTarget` _asenemy_interface))
  (bind _ascombat_interface (cast `CombatInterface` _returnvalue_2))
  (`CombatInterface.UpdateFacingTarget` _ascombat_interface (`Actor.K2_GetActorLocation` _returnvalue_3))
  (bind _returnvalue_4 (`CombatInterface.GetAttackMontages` _ascombat_interface))
  (set `self.TaggedMontage` (`KismetArrayLibrary.Array_Random` _returnvalue_4))
  (`AbilityTask_PlayMontageAndWait.CreatePlayMontageAndWaitProxy` "None" _taggedmontage_montage 1.0 "None" false
    (:`then`
      (`AbilityTask_WaitGameplayEvent.WaitGameplayEvent` _taggedmontage_montagetag null
        (:`EventReceived`
          (bind _ascombat_interface_2 (cast `CombatInterface` _returnvalue))
          (bind _returnvalue_5 (`CombatInterface.GetCombatSocketLocation` _ascombat_interface_2 _taggedmontage_montagetag))
          (bind _outoverlappingactors (`AuraAbilitySystemLibrary.GetLivePlayersWithRadius` self (`|MakeArray` _returnvalue) 45.0 _returnvalue_5))
          (for _array_element _outoverlappingactors
            (if (`AuraAbilitySystemLibrary.IsNotFriend` (`self.GetAvatarActorFromActorInfo`) _array_element)
              (`self.CauseDamage` _array_element))))))
    (:`OnCompleted`
      _)
    (:`OnInterrupted`
      _)
    (:`OnCancelled`
      _))
  (`self.K2_EndAbility`))