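; Enemy gameplay ability that summons random minions around the battlefield, using the Shaman summon montage.
; On activation it gets spawn locations, fires a summon gameplay cue at each, and plays the montage.
; The montage's attack event shuffles the locations and starts a delayed loop spawning AI-controlled minions one by one, then ends the ability.
; Each spawn increments the summoner's minion count via interface message; its destruction decrements it.
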(event `self.K2_ActivateAbility`
  (bind _returnvalue (+ (`|GetArrayItem` (`self.SpawnLocations`) (`self.SpawnLocationIndex`)) (0.0 0.0 70.0)))
  (set `self.SpawnLocationIndex` 0)
  (bind _returnvalue_2 (`self.GetSpawnLocations`))
  (bind _output_get (set `self.SpawnLocations` _returnvalue_2))
  (for _array_element _output_get
    (`self.K2_ExecuteGameplayCueWithParams` (struct :`TagName` "GameplayCue.Summon") (`AbilitySystemBlueprintLibrary.MakeGameplayCueParameters` 0.0 0.0 (struct) (struct) (struct) (struct) (struct) _array_element (0.0 0.0 0.0) null (`self.GetAvatarActorFromActorInfo`))))
  (`AbilityTask_PlayMontageAndWait.CreatePlayMontageAndWaitProxy` "None" "/Game/Assets/Enemies/Shaman/Animations/AM_Shaman_Summon.AM_Shaman_Summon"
    (:`then`
      (`AbilityTask_WaitGameplayEvent.WaitGameplayEvent` (struct :`TagName` "Montage.Attack.1") null
        (:`EventReceived`
          (`KismetArrayLibrary.Array_Shuffle` _output_get)
          (if (< (`self.SpawnLocationIndex`) (`KismetArrayLibrary.Array_Length` _output_get)) :!label _label
            (bind _returnvalue_3 (`|SpawnActorFromClass` (`self.GetRandomMinioClass`) (`KismetMathLibrary.MakeTransform` _returnvalue (`KismetMathLibrary.FindLookAtRotation` (`Actor.K2_GetActorLocation` (`self.GetAvatarActorFromActorInfo`)) _returnvalue)) "AlwaysSpawn" "MultiplyWithRoot" null null))
            (add `Actor.OnDestroyed` _returnvalue_3 (delegate `OnDestroyed_事件`))
            (`Pawn.SpawnDefaultController` _returnvalue_3)
            (message `CombatInterface.IncreaseMinionsCount` (`self.GetAvatarActorFromActorInfo`) 1)
            (`/Engine/EditorBlueprintResources/StandardMacros.IncrementInt` (`self.SpawnLocationIndex`)
              (:`  `
                (`KismetSystemLibrary.Delay` 0.2)
                (goto _label)))
            (else
              (`self.K2_EndAbility`))))))))

(event `OnDestroyed_事件`
  (params (DestroyedActor :type "Actor Object Reference"))
  (message `CombatInterface.IncreaseMinionsCount` (`self.GetAvatarActorFromActorInfo`) -1))