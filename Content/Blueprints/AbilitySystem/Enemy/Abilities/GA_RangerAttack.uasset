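; Gameplay ability for the Ranger enemy's ranged attack on its current combat target.
; On activation it gets the target through EnemyInterface, turns the avatar toward it through CombatInterface, and plays a random tagged attack montage.
; The montage's gameplay event tag triggers a projectile spawn at the target's location, read when the event arrives.
; The ability ends when the montage completes, is interrupted or is cancelled.
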(event `self.K2_ActivateAbility`
  (bind _returnvalue (`self.GetAvatarActorFromActorInfo`))
  (bind _taggedmontage_montage (break `TaggedMontage` (`self.TaggedMontage`)))
  (bind (_taggedmontage_montage_2 _taggedmontage_montagetag) (break `TaggedMontage` (`self.TaggedMontage`)))
  (bind _asenemy_interface (cast `EnemyInterface` _returnvalue))
  (bind _returnvalue_2 (`EnemyInterface.GetCombatTarget` _asenemy_interface))
  (set `self.CombatTarget` _returnvalue_2)
  (bind _ascombat_interface (cast `CombatInterface` _returnvalue))
  (`CombatInterface.UpdateFacingTarget` _ascombat_interface (`Actor.K2_GetActorLocation` (`self.CombatTarget`)))
  (bind _returnvalue_3 (`CombatInterface.GetAttackMontages` _ascombat_interface))
  (set `self.TaggedMontage` (`KismetArrayLibrary.Array_Random` _returnvalue_3))
  (`AbilityTask_PlayMontageAndWait.CreatePlayMontageAndWaitProxy` "None" _taggedmontage_montage 1.0 "None" false
    (:`then`
      (`AbilityTask_WaitGameplayEvent.WaitGameplayEvent` _taggedmontage_montagetag null
        (:`EventReceived`
          (`self.SpawnProjectile` (`Actor.K2_GetActorLocation` (`self.CombatTarget`))))))
    (:`OnCompleted`
      (`self.K2_EndAbility` :!label _label))
    (:`OnInterrupted`
      (goto _label))
    (:`OnCancelled`
      (goto _label))))