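; Arcane Shards gameplay ability that shows a magic circle, waits for a press, then erupts a series of damaging shards around the targeted point.
; On press it spawns a BP_PointCollection at the mouse hit to get ground points, their count set by ability level up to a cap, and plays the cast montage.
; The montage event commits the ability and starts a looping timer that fires one shard cue per point, applying radial damage with outward, pitched knockback.
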(event `self.K2_ActivateAbility`
  (`self.K2_CheckAbilityCost`)
  (if true
    (set `self.Count` 0)
    (set `self.Num Points` (`KismetMathLibrary.Min` (`self.GetAbilityLevel`) (`self.MaxNumPoints`)))
    (`|ExecutionSequence`
      (:`then_0`
        (`self.IsLocallyControlled`
          (:`True`
            (message `PlayerInterface.ShowMagicCircle` (`self.GetAvatarActorFromActorInfo`) null))))
      (:`then_1`
        (`AbilityTask_WaitInputPress.WaitInputPress` false
          (:`OnPress`
            (bind (_asynctaskproxy _datahandle) (`TargetDataUnderMouse.CreateTargetDataUnderMouse`)
              (:`ValidData`
                (`|ExecutionSequence`
                  (:`then_0`
                    (bind (_returnvalue_bblockinghit _returnvalue_binitialoverlap _returnvalue_time _returnvalue_distance _returnvalue_location _returnvalue_impactpoint) (`GameplayStatics.BreakHitResult` (`AbilitySystemBlueprintLibrary.GetHitResultFromTargetData` _datahandle)))
                    (bind _returnvalue (`|SpawnActorFromClass` "/Game/Blueprints/AbilitySystem/Aura/Abilities/Arcane/ArcaneShards/BP_PointCollection.BP_PointCollection_C" (`KismetMathLibrary.MakeTransform` _returnvalue_impactpoint) "AlwaysSpawn" "MultiplyWithRoot" null null))
                    (bind _output_get (set `self.PointCollections` _returnvalue))
                    (set `self.GroundPoints` (`PointCollection.GetGroundPoints` _output_get _returnvalue_impactpoint (`self.Num Points`) (`KismetMathLibrary.RandomFloatInRange` 0.0 360.0))))
                  (:`then_1`
                    (message `CombatInterface.UpdateFacingTarget` (`self.GetAvatarActorFromActorInfo`) _returnvalue_impactpoint))
                  (:`then_2`
                    (`AbilityTask_PlayMontageAndWait.CreatePlayMontageAndWaitProxy` "None" "/Game/Assets/Characters/Aura/Animations/Abilities/AM_Cast_ArcaneShards.AM_Cast_ArcaneShards"
                      (:`then`
                        (`AbilityTask_WaitGameplayEvent.WaitGameplayEvent` (struct :`TagName` "Event.Montage.ArcaneShards") null true
                          (:`EventReceived`
                            (bind _returnvalue_2 (`KismetSystemLibrary.K2_SetTimerDelegate` (delegate `SpawnShard`) (`self.ShardSpawnDeltaTime`) true false -1.0))
                            (set `self.ShardSpawnTimer` _returnvalue_2)
                            (message `PlayerInterface.HideMagicCircle` (`self.GetAvatarActorFromActorInfo`))
                            (`self.K2_CommitAbility`)))))))))))))))

(event `SpawnShard`
  (bind _returnvalue (`self.GetAvatarActorFromActorInfo`))
  (if (< (`self.Count`) (`self.Num Points`))
    (set `self.ShaedSpawnLocation` (`SceneComponent.K2_GetComponentLocation` (`|GetArrayItem` (`self.GroundPoints`) (`self.Count`))))
    (`/Engine/EditorBlueprintResources/StandardMacros.IncrementInt` (`self.Count`)
      (:`  `
        (`self.K2_ExecuteGameplayCueWithParams` (struct :`TagName` "GameplayCue.ArcaneShards") (`AbilitySystemBlueprintLibrary.MakeGameplayCueParameters` 0.0 0.0 (struct) (struct) (struct) (struct) (struct) (`self.ShaedSpawnLocation`)))
        (bind _outoverlappingactors (`AuraAbilitySystemLibrary.GetLivePlayersWithRadius` _returnvalue (`|MakeArray` _returnvalue) (`self.RadialDamageOuterRadius`) (`self.ShaedSpawnLocation`)))
        (bind _output_get (set `self.OverlappingPlayers` _outoverlappingactors))
        (for _array_element _output_get
          (bind _returnvalue_2 (- (`Actor.K2_GetActorLocation` _array_element) (`self.ShaedSpawnLocation`)))
          (`AuraAbilitySystemLibrary.ApplyDamageEffect` (`self.MakeDamageEffectParamsFromClassDefaults` _array_element (`self.ShaedSpawnLocation`) true _returnvalue_2 false _returnvalue_2 true 35.0)))))
    (else
      (`KismetSystemLibrary.K2_ClearAndInvalidateTimerHandle` (`self.ShardSpawnTimer`))
      (`Actor.K2_DestroyActor` (`self.PointCollections`))
      (`self.K2_EndAbility`))))