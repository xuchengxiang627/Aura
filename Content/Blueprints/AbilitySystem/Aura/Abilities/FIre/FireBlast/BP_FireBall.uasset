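; Fireball actor for the FireBlast ability that flies outward, returns to an assigned actor and explodes near it.
; On the server, one timeline moves it forward to an apex, then a second lerps it back toward that actor's live location.
; Within the explosion distance, it calls OnHit, applies radial GAS damage with outward knockback and death impulse to nearby live players except its owner, then destroys itself.
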(event `self.StartOutgoingTimeline`
  (bind _returnvalue (`self.GetOwner`))
  (bind _explosiondamageparams (`self.ExplosionDamageParams`))
  (bind _array (`|MakeArray` _returnvalue))
  (`/Engine/EditorBlueprintResources/ActorMacros.Switch Has Authority`
    (:`Authority`
      (set `self.Initial Location` (`self.K2_GetActorLocation`))
      (set `self.Apex Location` (+ (`self.Initial Location`) (* (`self.GetActorForwardVector`) (`self.TravelDiatance`))))
      (bind (_direction _outinggoing_track) (`Timeline|时间轴` :!via `PlayFromStart`)
        (:`Update`
          (`self.K2_SetActorLocation` (`KismetMathLibrary.VLerp` (`self.Initial Location`) (`self.Apex Location`) _outinggoing_track)))
        (:`Finished`
          (bind (_direction_2 _returnning_track) (`Timeline|时间轴_0` :!via `PlayFromStart`)
            (:`Update`
              (`self.K2_SetActorLocation` (`KismetMathLibrary.VLerp` (`self.K2_GetActorLocation` (`self.ReturnToActor`)) (`self.Apex Location`) _returnning_track))
              (if (<= (`KismetMathLibrary.Vector_Distance` (`self.K2_GetActorLocation` (`self.ReturnToActor`)) (`self.K2_GetActorLocation`)) (`self.ExplodeDistance`))
                (`self.OnHit`)
                (`KismetArrayLibrary.Array_Add` _array self)
                (bind _outoverlappingactors (`AuraAbilitySystemLibrary.GetLivePlayersWithRadius` _returnvalue _array 300.0 (`self.K2_GetActorLocation`)))
                (`AuraAbilitySystemLibrary.SetIsRadialDamageEffectParam` (`self.ExplosionDamageParams`) true 50.0 300.0 (`self.K2_GetActorLocation`))
                (for _array_element _outoverlappingactors
                  (`AuraAbilitySystemLibrary.SetTargetASCEffectParam` (`self.ExplosionDamageParams`) (`AbilitySystemBlueprintLibrary.GetAbilitySystemComponent` _array_element))
                  (bind _returnvalue_2 (- (`self.K2_GetActorLocation` _array_element) (`self.K2_GetActorLocation`)))
                  (`AuraAbilitySystemLibrary.SetKnockBackDirection` _explosiondamageparams _returnvalue_2 800.0)
                  (`AuraAbilitySystemLibrary.SetDeathImpulseDirection` _explosiondamageparams _returnvalue_2 600.0)
                  (`AuraAbilitySystemLibrary.ApplyDamageEffect` (`self.ExplosionDamageParams`)))
                (`self.K2_DestroyActor`)))))))))

(fn `UserConstructionScript`)