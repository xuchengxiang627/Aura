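; GA_FireBolt is a gameplay ability that casts a fire bolt toward the point under the mouse.
; On activation it commits, takes the mouse target data's hit location, and turns the avatar to face it through CombatInterface.
; It plays the cast montage, waits for its Event.Montage.FireBolt gameplay event to spawn the projectile from the weapon socket, and ends when the montage completes, blends out or is stopped.
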(event `self.K2_ActivateAbility`
  (`self.K2_CommitAbility`)
  (bind (_asynctaskproxy _datahandle) (`TargetDataUnderMouse.CreateTargetDataUnderMouse`)
    (:`ValidData`
      (set `self.ProjectileTargetLocation` (`.Location` (`GameplayStatics.BreakHitResult` (`AbilitySystemBlueprintLibrary.GetHitResultFromTargetData` _datahandle))))
      ;[1 1 1] 通过角色的MotionWarp组件控制角色转向Target
      (bind _ascombat_interface (cast `CombatInterface` (`self.GetAvatarActorFromActorInfo`))
        (:`then`
          (`CombatInterface.UpdateFacingTarget` _ascombat_interface (`self.ProjectileTargetLocation`)))
        (:`CastFailed`
          _))
      (`AbilityTask_PlayMontageAndWait.CreatePlayMontageAndWaitProxy` "None" "/Game/Assets/Characters/Aura/Animations/Abilities/AM_Cast_FireBolt.AM_Cast_FireBolt"
        (:`then`
          (`AbilityTask_WaitGameplayEvent.WaitGameplayEvent` (struct :`TagName` "Event.Montage.FireBolt") null ; 由蒙太奇进行动画通知触发Gameplay事件
            (:`EventReceived`
              (`self.SpawnProjectile` (`self.ProjectileTargetLocation`) (`BlueprintGameplayTagLibrary.MakeLiteralGameplayTag` (struct :`TagName` "CombatSocket.Weapon"))))))
        (:`OnCompleted`
          (`self.K2_EndAbility` :!label _label))
        (:`OnBlendOut`
          (goto _label))
        (:`OnInterrupted`
          (goto _label))
        (:`OnCancelled`
          (goto _label))))))