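; Flame pillar actor whose fire light flickers continuously from BeginPlay.
; ChooseTimeLine randomly picks one of two flame intensity timelines and plays it from the start.
; Each timeline scales BaseIntensity by its curve value to set the FireLight intensity, then calls ChooseTimeLine again when finished, giving an endless, varied flicker without using Tick.
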(event `self.ReceiveBeginPlay`
  (`self.ChooseTimeLine`))

(event `ChooseTimeLine`
  (switch `int` (`KismetMathLibrary.RandomIntegerInRange` 0 1)
    (:`0`
      (`self.StartTimeLine_1`))
    (:`1`
      (`self.StartTimeLine_2`))))

(event `StartTimeLine_1`
  (bind (_direction _falmeintensity) (`Timeline|FlameIntensityTimeLine_1` :!via `PlayFromStart`)
    (:`Update`
      (`LightComponent.SetIntensity` (`self.FireLight`) (* _falmeintensity (`self.BaseIntensity`))))
    (:`Finished`
      (`self.ChooseTimeLine`))))

(event `StartTimeLine_2`
  (bind (_direction _falmeintensity) (`Timeline|FlameIntensityTimeLine_2` :!via `PlayFromStart`)
    (:`Update`
      (`LightComponent.SetIntensity` (`self.FireLight`) (* _falmeintensity (`self.BaseIntensity`))))
    (:`Finished`
      (`self.ChooseTimeLine`))))

(fn `UserConstructionScript`)