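; Health potion pickup actor that applies an instant Gameplay Effect to any actor overlapping its sphere.
; On BeginPlay it starts sinusoidal movement and rotation and plays a ground impact sound at its location.
; Each Tick it moves itself to the calculated location and rotation; the motion math and effect application live in functions defined outside these graphs.
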(event `self.ReceiveBeginPlay`
  (`self.StartSinusoidalMovement`)
  (`self.StartRotation`)
  (`GameplayStatics.PlaySoundAtLocation` (`self.GroundImpactSound`) (`self.K2_GetActorLocation`) (struct) 1.0 1.0 0.0 null null null null))

(event `self.ReceiveTick`
  (params (DeltaSeconds :type "Float (single-precision)"))
  (`self.K2_SetActorLocationAndRotation` (`self.CalculatedLocation`) (`self.CalculatedRotation`)))

(event `self.Sphere.OnComponentBeginOverlap`
  (params (OverlappedComponent :type "PrimitiveComponent Object Reference") (OtherActor :type "Actor Object Reference") (OtherComp :type "PrimitiveComponent Object Reference") (OtherBodyIndex :type Integer) (bFromSweep :type Boolean) (SweepResult :type "HitResult Structure (by ref)"))
  (`self.ApplyEffectToTarget` OtherActor (`self.InstantGameplayEffectClass`)))

(fn `UserConstructionScript`)